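; Grid inventory that stores stackable items in a slot array sized from width and row count, filled with empty slots on BeginPlay.
; AddItem places one item via HasPlaceableSlot, which searches for a partial stack from the selected row with wraparound, then falls back to the selected slot or first empty one.
; Removal works by index or by type across stacks, optionally selected slot first, and fires InventoryChanged, as does adding.
; Query helpers report slot contents and item availability.
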(event `self.ReceiveBeginPlay`
  (`/Engine/EditorBlueprintResources/StandardMacros.ForLoopConditional` 0 "NewEnumerator0" (* (`self.InventoryWidth`) (`self.InventoryRowCount`))
    (:`LoopBody`
      (`KismetArrayLibrary.Array_Add` (`self.Items`) (make `/Game/DataAssets/PrimaryDataAssets/Inventory/SInventorySlot` null)))))

(fn `AddItem`
  (params (ItemToAdd :type "/Game/DataAssets/PrimaryDataAssets/Inventory/PDA_Base_InventoryItem Object Reference"))
  (returns (ItemAdded :type Boolean))
  (bind (_hasslot _inventoryindex) (`self.HasPlaceableSlot` ItemToAdd))
  (if _hasslot
    (bind (_output_itemdata _output_itemamount) (break `/Game/DataAssets/PrimaryDataAssets/Inventory/SInventorySlot` (`|GetArrayItem` (`self.Items`) _inventoryindex)))
    (`KismetArrayLibrary.Array_Set` (`self.Items`) _inventoryindex (make `/Game/DataAssets/PrimaryDataAssets/Inventory/SInventorySlot` ItemToAdd (+ _output_itemamount 1)))
    (`self.InventoryChanged`)
    (return true)
    (else
      (return false))))

(fn `ContainsItem`
  (params (ItemType :type "/Game/DataAssets/PrimaryDataAssets/Inventory/PDA_Base_InventoryItem Object Reference"))
  (returns (HasItem :type Boolean))
  (locals (TestItem :type "/Game/DataAssets/PrimaryDataAssets/Inventory/PDA_Base_InventoryItem Object Reference"))
  (set `local.TestItem` ItemType)
  (for _array_element (`self.Items`)
    (bind (_itemdata _itemamount) (break `/Game/DataAssets/PrimaryDataAssets/Inventory/SInventorySlot` _array_element))
    (if (and (== _itemdata (`local.TestItem`)) (> _itemamount 0))
      (return true)))
  (return false))

(fn `ContainsItemAtIndex`
  (params (InventoryIndex :type Integer))
  (returns (HasItem :type Boolean) (Item :type "/Game/DataAssets/PrimaryDataAssets/Inventory/PDA_Base_InventoryItem Object Reference"))
  (locals (TestItem :type "/Game/DataAssets/PrimaryDataAssets/Inventory/PDA_Base_InventoryItem Object Reference"))
  (bind (_output_itemdata _output_itemamount) (break `/Game/DataAssets/PrimaryDataAssets/Inventory/SInventorySlot` (`|GetArrayItem` (`self.Items`) InventoryIndex)))
  (if (or (not (`KismetSystemLibrary.IsValid` _output_itemdata)) (<= _output_itemamount 0))
    (return false null)
    (else
      (return true _output_itemdata))))

(fn `GetInventorySlotAtIndex`
  (params (ItemIndex :type Integer))
  (returns (InventorySlot :type "/Game/DataAssets/PrimaryDataAssets/Inventory/SInventorySlot Structure"))
  (return (`|GetArrayItem` (`self.Items`) ItemIndex)))

(fn `GetItemDataAtIndex`
  (params (InventoryIndex :type Integer))
  (returns (InventoryItem :type "/Game/DataAssets/PrimaryDataAssets/Inventory/PDA_Base_InventoryItem Object Reference") (NullItem :type Boolean))
  (bind (_output_itemdata _output_itemamount) (break `/Game/DataAssets/PrimaryDataAssets/Inventory/SInventorySlot` (`|GetArrayItem` (`self.Items`) InventoryIndex)))
  (return _output_itemdata (or (== _output_itemdata null) (== _output_itemamount 0))))

(fn `GetSelectedItem`
  (returns (Item :type "/Game/DataAssets/PrimaryDataAssets/Inventory/PDA_Base_InventoryItem Object Reference"))
  (bind _output_itemdata (break `/Game/DataAssets/PrimaryDataAssets/Inventory/SInventorySlot` (`|GetArrayItem` (`self.Items`) (`self.SelectedIndex`))))
  (return _output_itemdata))

(fn `Has Item`
  (params (ItemToCheck :type "/Game/DataAssets/PrimaryDataAssets/Inventory/PDA_Base_InventoryItem Object Reference") (AmountNeeded :type Integer))
  (returns (NewParam :type Boolean))
  (locals (AmountNecessary :type Integer) (CheckingItem :type "/Game/DataAssets/PrimaryDataAssets/Inventory/PDA_Base_InventoryItem Object Reference"))
  (bind _amountnecessary (`local.AmountNecessary`))
  (set `local.CheckingItem` ItemToCheck)
  (set `local.AmountNecessary` AmountNeeded)
  (for _array_element (`self.Items`)
    (bind (_itemdata _itemamount) (break `/Game/DataAssets/PrimaryDataAssets/Inventory/SInventorySlot` _array_element))
    (if (== (`local.CheckingItem`) _itemdata)
      (if (>= _itemamount _amountnecessary)
        (return true)
        (else
          (set `local.AmountNecessary` (- _amountnecessary _itemamount))))))
  (return false))

(fn `HasPlaceableSlot`
  (params (Item :type "/Game/DataAssets/PrimaryDataAssets/Inventory/PDA_Base_InventoryItem Object Reference"))
  (returns (HasSlot :type Boolean) (InventoryIndex :type Integer))
  (locals (EmptySlot :type Integer) (Index :type Integer) (HasEmptySlot :type Boolean))
  (bind _items (`self.Items`))
  (bind _selectedindex (`self.SelectedIndex`))
  (bind _selectedindex_2 (`self.SelectedIndex`))
  (bind _index (`local.Index`))
  (bind (_output_itemdata _output_itemamount) (break `/Game/DataAssets/PrimaryDataAssets/Inventory/SInventorySlot` (`|GetArrayItem` (`self.Items`) _selectedindex)))
  (bind (_output_itemdata_2 _output_itemamount_2) (break `/Game/DataAssets/PrimaryDataAssets/Inventory/SInventorySlot` (`|GetArrayItem` _items _index)))
  (set `local.Index` (- _selectedindex_2 (mod _selectedindex_2 (`self.InventoryWidth`))))
  (`/Engine/EditorBlueprintResources/StandardMacros.ForLoopConditional` 0 "NewEnumerator0" (`KismetArrayLibrary.Array_Length` _items)
    (:`LoopBody`
      (if (`KismetSystemLibrary.IsValid` _output_itemdata_2)
        (if (and (== _output_itemdata_2 Item) (< _output_itemamount_2 (`/Game/DataAssets/PrimaryDataAssets/Inventory/PDA_Base_InventoryItem.MaxStack` Item)))
          (return true _index)
          (else
            _))
        (elif (not (`local.HasEmptySlot`))
          (set `local.EmptySlot` _index)
          (set `local.HasEmptySlot` true)))
      (`/Engine/EditorBlueprintResources/StandardMacros.IncrementInt` _index
        (:`  `
          (if (>= (`local.Index`) (* (`self.InventoryWidth`) (`self.InventoryRowCount`)))
            (set `local.Index` 0)))))
    (:`Completed`
      (if (`KismetSystemLibrary.IsValid` _output_itemdata)
        (if (and (== Item _output_itemdata) (< _output_itemamount (`/Game/DataAssets/PrimaryDataAssets/Inventory/PDA_Base_InventoryItem.MaxStack` _output_itemdata)))
          (return true _selectedindex)
          (elif (`local.HasEmptySlot`)
            (return true (`local.EmptySlot`))
            (else
              (return false 0))))
        (else
          (return true _selectedindex))))))

(fn `InventorySize`
  (returns (Size :type Integer))
  (return (* (`self.InventoryWidth`) (`self.InventoryRowCount`))))

(fn `Remove Item By Index`
  (params (InventoryIndex :type Integer) (AmountToRemove :type Integer :default 1))
  (returns (Removed :type Boolean))
  (locals (CurrentInvIndex :type Integer))
  (bind _items (`self.Items`))
  (bind _currentinvindex (`local.CurrentInvIndex`))
  (bind (_output_itemdata _output_itemamount) (break `/Game/DataAssets/PrimaryDataAssets/Inventory/SInventorySlot` (`|GetArrayItem` _items _currentinvindex)))
  (bind _output_get (set `local.CurrentInvIndex` InventoryIndex))
  (bind (_output_itemdata_2 _output_itemamount_2) (break `/Game/DataAssets/PrimaryDataAssets/Inventory/SInventorySlot` (`|GetArrayItem` (`self.Items`) _output_get)))
  (if (or (> AmountToRemove _output_itemamount_2) (not (`KismetSystemLibrary.IsValid` _output_itemdata_2)))
    (return false)
    (else
      (if (== _output_itemamount_2 AmountToRemove)
        (`KismetArrayLibrary.Array_Set` _items _currentinvindex (make `/Game/DataAssets/PrimaryDataAssets/Inventory/SInventorySlot` null))
        (else
          (`KismetArrayLibrary.Array_Set` _items _currentinvindex (make `/Game/DataAssets/PrimaryDataAssets/Inventory/SInventorySlot` _output_itemdata (- _output_itemamount AmountToRemove)))))
      (`self.InventoryChanged`))))

(fn `RemoveItemByType`
  (params (StartAtSelectedItem :type Boolean) (ItemToRemove :type "/Game/DataAssets/PrimaryDataAssets/Inventory/PDA_Base_InventoryItem Object Reference") (AmountToRemove :type Integer))
  (returns (CanRemove :type Boolean))
  (locals (StartSelected :type Boolean) (RemovingItem :type "/Game/DataAssets/PrimaryDataAssets/Inventory/PDA_Base_InventoryItem Object Reference") (RemoveAmount :type Integer) (CurrentIndex :type Integer))
  (bind _removeamount (`local.RemoveAmount`))
  (bind (_output_itemdata _output_itemamount) (break `/Game/DataAssets/PrimaryDataAssets/Inventory/SInventorySlot` (`|GetArrayItem` (`self.Items`) (`self.SelectedIndex`))))
  (set `local.StartSelected` StartAtSelectedItem)
  (set `local.RemovingItem` ItemToRemove)
  (set `local.RemoveAmount` AmountToRemove)
  (if (`local.StartSelected`)
    ;[1 1 1] If starting with selected slot, check that first
    (if (== _output_itemdata (`local.RemovingItem`))
      (if (> _output_itemamount (`local.RemoveAmount`))
        (`KismetArrayLibrary.Array_Set` (`self.Items`) (`self.SelectedIndex`) (make `/Game/DataAssets/PrimaryDataAssets/Inventory/SInventorySlot` (`local.RemovingItem`) (- _output_itemamount (`local.RemoveAmount`))))
        (`self.InventoryChanged`)
        (return true)
        (else
          (bind _output_get (set `local.RemoveAmount` (- (`local.RemoveAmount`) _output_itemamount)))
          (`KismetArrayLibrary.Array_Set` (`self.Items`) (`self.SelectedIndex`) (make `/Game/DataAssets/PrimaryDataAssets/Inventory/SInventorySlot` null))
          (`self.InventoryChanged`)
          (if (<= _output_get 0)
            (return true)
            (else
              (bind _index (`/Engine/EditorBlueprintResources/StandardMacros.ForLoopConditional` 0 "NewEnumerator0" (`KismetArrayLibrary.Array_Length` (`self.Items`)) :!label _label)
                (:`LoopBody`
                  (set `local.CurrentIndex` _index)
                  ;[1 1 1] If checked selected, dont double check
                  (if (`local.StartSelected`)
                    (if (not (== _index (`self.SelectedIndex`)))
                      (bind (_output_itemdata_2 _output_itemamount_2) (break `/Game/DataAssets/PrimaryDataAssets/Inventory/SInventorySlot` (`|GetArrayItem` (`self.Items`) _index)))
                      (if (== _output_itemdata_2 (`local.RemovingItem`)) :!label _label_2
                        (if (> _output_itemamount_2 (`local.RemoveAmount`))
                          ;[1 1 1] If the current item's amount is greater, adjust that item, and then return true
                          (`KismetArrayLibrary.Array_Set` (`self.Items`) (`local.CurrentIndex`) (make `/Game/DataAssets/PrimaryDataAssets/Inventory/SInventorySlot` (`local.RemovingItem`) (- _output_itemamount_2 _removeamount)))
                          (`self.InventoryChanged`)
                          (return true)
                          (else
                            ;[1 1 1] If current item is equal to, or less than removed amount, reset slot & adjust removed amount with new amount. If the amount has been found, return true
                            (set `local.RemoveAmount` (- _removeamount _output_itemamount_2))
                            (`KismetArrayLibrary.Array_Set` (`self.Items`) (`local.CurrentIndex`) (make `/Game/DataAssets/PrimaryDataAssets/Inventory/SInventorySlot` null))
                            (if (== (`local.RemoveAmount`) 0)
                              (`self.InventoryChanged`)
                              (return true))))))
                    (else
                      (goto _label_2))))
                (:`Completed`
                  (`KismetSystemLibrary.PrintString` "There was an error in removing the item")
                  (return false))))))))
    (else
      (goto _label))))

(fn `StartingRowIndex`
  (returns (Index :type Integer))
  (bind _selectedindex (`self.SelectedIndex`))
  (return (- _selectedindex (mod _selectedindex (`self.InventoryWidth`)))))