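; Base interactable that hands player control over to itself when interacted with.
; On interaction it disables further interaction and switches off the player character's inputs using that character's DisableOnInteract bitmask.
; It then eases the camera view to itself, waits for the one-second blend and has the player controller possess it.
; The file contains no logic for returning control to the character.
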(event `self.PerformInteraction`
  (set `self.CanInteract` false)
  (bind _asbp_player_char (cast `/Game/Character/BP_PlayerChar` (`GameplayStatics.GetPlayerPawn` 0)))
  (`/Game/Character/BP_PlayerChar.Toggle Inputs` _asbp_player_char false (`/Game/Character/BP_PlayerChar.DisableOnInteract` _asbp_player_char))
  (`PlayerController.SetViewTargetWithBlend` (`GameplayStatics.GetPlayerController` 0) self 1.0 "VTBlend_EaseInOut" 3.0 false)
  (`KismetSystemLibrary.Delay` 1.0)
  (`Controller.Possess` (`GameplayStatics.GetPlayerController` 0) self))

(fn `UserConstructionScript`
  (`parent.UserConstructionScript`))