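; Boid manager that drives fish schooling, grouping registered boids by fish type.
; Each tick it compares every pair within a type using squared distances against perception and avoidance radii, summing heading, center and separation.
; It passes these sums and the neighbor count to each boid, then calls PerformMovement on all.
; The separation sum, unlike the others, is not reset between boids in the loop.
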(event `self.ReceiveTick`
  (params (DeltaSeconds :type "Float (single-precision)"))
  (`self.UpdateBoids`))

(fn `AddBoid`
  (params (Boid :type "/Game/Blueprints/Interactables/TankBlueprints/BP_Fish Object Reference"))
  (bind _fishtype (`/Game/DataAssets/PrimaryDataAssets/PDA_Animal_Fish.FishType` (`/Game/Blueprints/Interactables/TankBlueprints/BP_Fish.FishData` Boid)))
  (for (_array_element _array_index) (`self.MyBoids`)
    (if (`|EnumEquality` (`.FishType_7_D81D9C8440ECE63A1A1CA7A31224A980` (break `/Game/Blueprints/Struct_BoidType` _array_element)) _fishtype)
      (bind (_output_fishtype _output_boids) (break `/Game/Blueprints/Struct_BoidType` (`|GetArrayItem` (`self.MyBoids`) _array_index)))
      (`KismetArrayLibrary.Array_Add` _output_boids Boid)
      (return)))
  (`KismetArrayLibrary.Array_Add` (`self.MyBoids`) (make `/Game/Blueprints/Struct_BoidType` _fishtype (`|MakeArray` Boid))))

(fn `CalculateBoidVals`
  (params (UpdateBoids :type "/Game/Blueprints/Struct_BoidType Structure"))
  (locals (CurrentIndex :type Integer) (Offset :type "Vector Structure") (SqrDis :type "Float (double-precision)") (NumFlocks :type Integer) (FlockHead :type "Vector Structure") (FlockCenter :type "Vector Structure") (AvoidRad :type "Float (double-precision)") (SeparationHeading :type "Vector Structure") (PerceptionDis :type "Float (double-precision)"))
  (bind (_fishtype _boids) (break `/Game/Blueprints/Struct_BoidType` UpdateBoids))
  (bind _perceptiondis (`local.PerceptionDis`))
  (bind _avoidrad (`local.AvoidRad`))
  (bind _returnvalue (`KismetArrayLibrary.Array_Length` _boids))
  (bind _index (`/Engine/EditorBlueprintResources/StandardMacros.ForLoopConditional` 0 "NewEnumerator0" _returnvalue)
    (:`LoopBody`
      (set `local.NumFlocks` 0)
      (set `local.FlockHead` (0.0 0.0 0.0))
      (set `local.FlockCenter` (0.0 0.0 0.0))
      (bind _fishdata (`/Game/Blueprints/Interactables/TankBlueprints/BP_Fish.FishData` (`|GetArrayItem` _boids _index)))
      (set `local.AvoidRad` (`/Game/DataAssets/PrimaryDataAssets/PDA_Animal_Fish.avoidanceRadius` _fishdata))
      (set `local.PerceptionDis` (`/Game/DataAssets/PrimaryDataAssets/PDA_Animal_Fish.perceptionRadius` _fishdata))
      (bind _index_2 (`/Engine/EditorBlueprintResources/StandardMacros.ForLoopConditional` 0 "NewEnumerator0" _returnvalue)
        (:`LoopBody`
          (if (not (== _index_2 _index))
            (bind _output (`|GetArrayItem` _boids _index_2))
            (bind _pos (`/Game/Blueprints/Interactables/TankBlueprints/BP_Fish.Pos` _output))
            (bind _output_get (set `local.Offset` (- _pos (`/Game/Blueprints/Interactables/TankBlueprints/BP_Fish.Pos` (`|GetArrayItem` _boids _index)))))
            (bind _output_get_2 (set `local.SqrDis` (+ (* (.x _output_get) (.x _output_get)) (* (.y _output_get) (.y _output_get)) (* (.z _output_get) (.z _output_get)))))
            (if (< _output_get_2 (* _perceptiondis _perceptiondis))
              (`/Engine/EditorBlueprintResources/StandardMacros.IncrementInt` (`local.NumFlocks`)
                (:`  `
                  (set `local.FlockHead` (+ (`local.FlockHead`) (`/Game/Blueprints/Interactables/TankBlueprints/BP_Fish.Forward` _output)))
                  (set `local.FlockCenter` (+ (`local.FlockCenter`) _pos))
                  (if (< _output_get_2 (* _avoidrad _avoidrad))
                    (set `local.SeparationHeading` (- (`local.SeparationHeading`) (/ (`local.Offset`) (`local.SqrDis`))))))))))
        (:`Completed`
          (`/Game/Blueprints/Interactables/TankBlueprints/BP_Fish.SetSchoolVals` (`|GetArrayItem` _boids _index) (`local.FlockHead`) (`local.FlockCenter`) (`local.SeparationHeading`) (`local.NumFlocks`)))))))

(fn `UpdateBoids`
  (bind _myboids (`self.MyBoids`))
  (for _array_element _myboids
    (`self.CalculateBoidVals` _array_element))
  (for _array_element_2 _myboids
    (for _array_element_3 (`.Boids_5_97B907D14A8B3FE92AC351AE14E41473` (break `/Game/Blueprints/Struct_BoidType` _array_element_2))
      (`/Game/Blueprints/Interactables/TankBlueprints/BP_Fish.PerformMovement` _array_element_3))))