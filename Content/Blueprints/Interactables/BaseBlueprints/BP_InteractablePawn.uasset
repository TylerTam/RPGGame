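; Base interactable pawn that takes over view and control when the player interacts, with a camera movable inside a tank.
; Interaction disables player inputs, blends the view, then possesses this pawn; cancel calls back to the player and an empty InteractionStopped hook.
; Camera movement sphere-traces X and Y separately to stay in bounds, and CameraLerpComplete restores its start position.
; Inventory and quick-select inputs are forwarded to the player character.
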(event `self.ReceiveBeginPlay`
  (add `self.Interacted` (delegate `PerformInteraction`))
  (set `self.CameraStartPos` (`SceneComponent.RelativeLocation` (`self.MovementPart`))))

(event `PerformInteraction`
  (set `self.CanInteract` false)
  (bind _asbp_player_char (cast `/Game/Character/BP_PlayerChar` (`GameplayStatics.GetPlayerPawn` 0)))
  (`/Game/Character/BP_PlayerChar.Toggle Inputs` _asbp_player_char false (`/Game/Character/BP_PlayerChar.DisableOnInteract` _asbp_player_char))
  (`PlayerController.SetViewTargetWithBlend` (`GameplayStatics.GetPlayerController` 0) self 1.0 "VTBlend_EaseInOut" 3.0 false)
  (`KismetSystemLibrary.Delay` 1.0)
  (`Controller.Possess` (`GameplayStatics.GetPlayerController` 0) self))

(event `OnInteract`
  (params (Instigator :type "Actor Object Reference"))
  (bind _asbp_player_char (cast `/Game/Character/BP_PlayerChar` Instigator)
    (:`then`
      (set `self.PlayerPawn` _asbp_player_char))
    (:`CastFailed`
      _))
  (bind _aspawn (cast `Pawn` Instigator))
  (set `self.OriginalPawn` _aspawn)
  (if (`self.CanInteract`)
    (if (`self.CheckInteractable`)
      (`self.Interacted`))))

(event `EnhancedInput|/Game/Input/EnhancedInput/IA_Move`
  (params (ActionValue :type "Vector2D Structure") (ElapsedSeconds :type "Float (double-precision)") (TriggeredSeconds :type "Float (double-precision)") (InputAction :type "InputAction Object Reference" :default "/Game/Input/EnhancedInput/IA_Move.IA_Move"))
  (:`Triggered`
    (`self.MoveCamera` ActionValue)))

(event `EnhancedInput|/Game/Input/EnhancedInput/IA_Cancel`
  (params (ActionValue :type Boolean) (ElapsedSeconds :type "Float (double-precision)") (TriggeredSeconds :type "Float (double-precision)") (InputAction :type "InputAction Object Reference" :default "/Game/Input/EnhancedInput/IA_Cancel.IA_Cancel"))
  (:`Triggered`
    (set `self.CanInteract` true)
    (bind _asbp_player_char (cast `/Game/Character/BP_PlayerChar` (`self.OriginalPawn`)))
    (`/Game/Character/BP_PlayerChar.CancelPressedEvent` _asbp_player_char)
    (`self.InteractionStopped`)))

(event `EnhancedInput|/Game/Input/EnhancedInput/IA_QuickSelectDir`
  (params (ActionValue :type "Float (double-precision)") (ElapsedSeconds :type "Float (double-precision)") (TriggeredSeconds :type "Float (double-precision)") (InputAction :type "InputAction Object Reference" :default "/Game/Input/EnhancedInput/IA_QuickSelectDir.IA_QuickSelectDir"))
  (:`Triggered`
    (`/Game/Character/BP_PlayerChar.SelectedItemChange` (`self.PlayerPawn`) (`KismetMathLibrary.FTrunc` (`KismetMathLibrary.SignOfFloat` ActionValue)))))

(event `EnhancedInput|/Game/Input/EnhancedInput/IA_QuickSelectRow`
  (params (ActionValue :type "Float (double-precision)") (ElapsedSeconds :type "Float (double-precision)") (TriggeredSeconds :type "Float (double-precision)") (InputAction :type "InputAction Object Reference" :default "/Game/Input/EnhancedInput/IA_QuickSelectRow.IA_QuickSelectRow"))
  (:`Triggered`
    (`/Game/Character/BP_PlayerChar.SelectedRowChanged` (`self.PlayerPawn`) (`KismetMathLibrary.FTrunc` (`KismetMathLibrary.SignOfFloat` ActionValue)))))

(event `EnhancedInput|/Game/Input/EnhancedInput/IA_UseSelected`
  (params (ActionValue :type Boolean) (ElapsedSeconds :type "Float (double-precision)") (TriggeredSeconds :type "Float (double-precision)") (InputAction :type "InputAction Object Reference" :default "/Game/Input/EnhancedInput/IA_UseSelected.IA_UseSelected"))
  (:`Triggered`
    (`/Game/Character/BP_PlayerChar.UseSelectedItemFromPawn` (`self.PlayerPawn`) self)))

(event `EnhancedInput|/Game/Input/EnhancedInput/IA_OpenInventory`
  (params (ActionValue :type Boolean) (ElapsedSeconds :type "Float (double-precision)") (TriggeredSeconds :type "Float (double-precision)") (InputAction :type "InputAction Object Reference" :default "/Game/Input/EnhancedInput/IA_OpenInventory.IA_OpenInventory"))
  (:`Triggered`
    (`/Game/Character/BP_PlayerChar.OpenInventory` (`self.PlayerPawn`))))

(fn `CameraLerpComplete`
  (`SceneComponent.K2_SetRelativeLocation` (`self.MovementPart`) (`self.CameraStartPos`) false false))

(fn `CheckInteractable`
  (returns (CanInteract :type Boolean))
  (return true))

(fn `InteractionStopped`)

(fn `KeepInteractableRef`
  (returns (HoldRef :type Boolean))
  (return (`self.KeepAsRef`)))

(fn `MoveCamera`
  (params (Dir :type "Vector2D Structure"))
  (locals (NewLocation :type "Vector Structure") (DirX :type "Float (double-precision)" :default 0.0) (DirY :type "Float (double-precision)" :default 0.0))
  (bind (_tankmovespeed_x _tankmovespeed_y) (`KismetMathLibrary.BreakVector` (`self.TankMoveSpeed`)))
  (bind _movementpart (`self.MovementPart`))
  (bind (_returnvalue_x _returnvalue_y _returnvalue_z) (`KismetMathLibrary.BreakVector` (`SceneComponent.K2_GetComponentLocation` _movementpart)))
  (bind _returnvalue (`SceneComponent.K2_GetComponentLocation` (`self.MovementPart`)))
  (set `local.DirX` (* Dir_X _tankmovespeed_x))
  (set `local.DirY` (* Dir_Y _tankmovespeed_y))
  (set `local.NewLocation` _returnvalue)
  ;[1 1 1] To stop the camera from leaving the tank
  (bind (_outhit _returnvalue_2) (`KismetSystemLibrary.SphereTraceSingle` :`Start` _returnvalue :`End` (`KismetMathLibrary.MakeVector` (+ (`local.DirX`) _returnvalue_x) _returnvalue_y _returnvalue_z) :`Radius` 0.25 :`TraceChannel` "TraceTypeQuery3" :`bIgnoreSelf` false))
  (if (not _returnvalue_2)
    (set `local.NewLocation` (+ (`local.NewLocation`) (`KismetMathLibrary.MakeVector` (`local.DirX`)))))
  (bind (_outhit_2 _returnvalue_3) (`KismetSystemLibrary.SphereTraceSingle` :`Start` (`SceneComponent.K2_GetComponentLocation` (`self.MovementPart`)) :`End` (`KismetMathLibrary.MakeVector` _returnvalue_x (+ _returnvalue_y (`local.DirY`)) _returnvalue_z) :`Radius` 0.25 :`TraceChannel` "TraceTypeQuery3" :`bIgnoreSelf` false))
  (if (not _returnvalue_3)
    (set `local.NewLocation` (+ (`local.NewLocation`) (`KismetMathLibrary.MakeVector` 0.0 (`local.DirY`)))))
  (`SceneComponent.K2_SetWorldLocation` _movementpart (`local.NewLocation`) true false))

(fn `UserConstructionScript`)