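; BP_Interactable is a base Blueprint for interactable objects, with stub hooks for child classes to override.
; OnInteract fires the Interacted dispatcher when CanInteract and CheckInteractable both pass; BeginPlay binds the empty PerformInteraction event to that dispatcher.
; CheckInteractable returns true by default, StopInteraction sets CanInteract back to true, and KeepInteractableRef exposes the KeepAsRef flag.
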(event `self.ReceiveBeginPlay`
  (add `self.Interacted` (delegate `PerformInteraction`)))

(event `PerformInteraction`)

(event `OnInteract`
  (params (Instigator :type "Actor Object Reference"))
  (if (`self.CanInteract`)
    (if (`self.CheckInteractable`)
      (`self.Interacted`))))

(fn `CheckInteractable`
  (returns (CanInteract :type Boolean))
  (return true))

(fn `KeepInteractableRef`
  (returns (HoldRef :type Boolean))
  (return (`self.KeepAsRef`)))

(fn `StopInteraction`
  (set `self.CanInteract` true))

(fn `UserConstructionScript`)