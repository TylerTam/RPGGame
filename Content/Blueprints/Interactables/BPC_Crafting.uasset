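; Interactable crafting station that turns items from the interacting actor's BP_Inventory into a timed recipe output.
; On interact while idle, it matches the selected item to a recipe's main item, checks and consumes all ingredients, then starts a countdown on Tick.
; When the timer runs out, a PaperSprite shows the product, and the next interact hides it and adds the items to that actor's inventory.
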(event `self.ReceiveTick`
  (params (DeltaSeconds :type "Float (single-precision)"))
  (`self.Update Timer` DeltaSeconds))

(event `self.OnInteract`
  (params (Instigator :type "Actor Object Reference"))
  (bind _returnvalue (`self.GetComponentByClass` Instigator "/Game/Blueprints/Inventory/BP_Inventory.BP_Inventory_C"))
  (bind (_produceditem_itemdata _produceditem_itemamount) (break `/Game/DataAssets/PrimaryDataAssets/Inventory/SInventorySlot` (`/Game/DataAssets/PrimaryDataAssets/Crafting/PDA_CraftingRecipe.ProducedItem` (`self.CurrentRecipe`))))
  (if (`KismetSystemLibrary.IsValid` _returnvalue)
    (if (`self.CreatingItem`)
      (if (<= (`self.CurrentTimer`) 0.0)
        (`SceneComponent.SetVisibility` (`self.PaperSprite`) false false)
        (set `self.CreatingItem` false)
        (bind _index (`/Engine/EditorBlueprintResources/StandardMacros.ForLoopConditional` 0 "NewEnumerator0" _produceditem_itemamount)
          (:`LoopBody`
            (`KismetSystemLibrary.PrintString` (`KismetStringLibrary.Concat_StrStr` (`KismetStringLibrary.Conv_IntToString` _index) " | " (`KismetStringLibrary.Conv_IntToString` _produceditem_itemamount)))
            (`/Game/Blueprints/Inventory/BP_Inventory.AddItem` _returnvalue _produceditem_itemdata))))
      (else
        (bind _recipe (`self.Get Possible Recipe` (`/Game/Blueprints/Inventory/BP_Inventory.GetSelectedItem` _returnvalue)))
        (if (`KismetSystemLibrary.IsValid` _recipe)
          (if (`self.CanUseRecipe` _returnvalue _recipe)
            (`self.UseRecipe` _returnvalue _recipe)
            (set `self.CreatingItem` true)
            (bind _output_get (set `self.CurrentRecipe` _recipe))
            (set `self.CurrentTimer` (`/Game/DataAssets/PrimaryDataAssets/Crafting/PDA_CraftingRecipe.TimeToCreate` _output_get))))))))

(fn `CanUseRecipe`
  (params (Inventory :type "/Game/Blueprints/Inventory/BP_Inventory Object Reference") (CheckingRecipe :type "/Game/DataAssets/PrimaryDataAssets/Crafting/PDA_CraftingRecipe Object Reference"))
  (returns (CanUse :type Boolean))
  (locals (CurrentInvetory :type "/Game/Blueprints/Inventory/BP_Inventory Object Reference") (Recipe :type "/Game/DataAssets/PrimaryDataAssets/Crafting/PDA_CraftingRecipe Object Reference"))
  (bind _recipe (`local.Recipe`))
  (bind (_mainitem_itemdata _mainitem_itemamount) (break `/Game/DataAssets/PrimaryDataAssets/Inventory/SInventorySlot` (`/Game/DataAssets/PrimaryDataAssets/Crafting/PDA_CraftingRecipe.MainItem` _recipe)))
  (set `local.Recipe` CheckingRecipe)
  (bind _output_get (set `local.CurrentInvetory` Inventory))
  (if (`/Game/Blueprints/Inventory/BP_Inventory.Has Item` _output_get _mainitem_itemdata _mainitem_itemamount)
    (for _array_element (`/Game/DataAssets/PrimaryDataAssets/Crafting/PDA_CraftingRecipe.SecondaryIngrediants` _recipe)
      (bind (_itemdata _itemamount) (break `/Game/DataAssets/PrimaryDataAssets/Inventory/SInventorySlot` _array_element))
      (if (not (`/Game/Blueprints/Inventory/BP_Inventory.Has Item` (`local.CurrentInvetory`) _itemdata _itemamount))
        (return false)))
    (return true)
    (else
      (return false))))

(fn `Get Possible Recipe`
  (params (Item :type "/Game/DataAssets/PrimaryDataAssets/Inventory/PDA_Base_InventoryItem Object Reference"))
  (returns (Recipe :type "/Game/DataAssets/PrimaryDataAssets/Crafting/PDA_CraftingRecipe Object Reference"))
  (for _array_element (`self.Recipes`)
    (bind _mainitem_itemdata (break `/Game/DataAssets/PrimaryDataAssets/Inventory/SInventorySlot` (`/Game/DataAssets/PrimaryDataAssets/Crafting/PDA_CraftingRecipe.MainItem` _array_element)))
    (if (== _mainitem_itemdata Item)
      (return _array_element)))
  (return null))

(fn `Update Timer`
  (params (DeltaTime :type "Float (double-precision)"))
  (bind _currenttimer (`self.CurrentTimer`))
  (bind _papersprite (`self.PaperSprite`))
  (bind _produceditem_itemdata (break `/Game/DataAssets/PrimaryDataAssets/Inventory/SInventorySlot` (`/Game/DataAssets/PrimaryDataAssets/Crafting/PDA_CraftingRecipe.ProducedItem` (`self.CurrentRecipe`))))
  (if (`self.CreatingItem`)
    (if (> _currenttimer 0.0)
      (set `self.CurrentTimer` (- _currenttimer DeltaTime))
      (if (< (`self.CurrentTimer`) 0.0)
        (`SceneComponent.SetVisibility` _papersprite true false)
        (`PaperSpriteComponent.SetSprite` _papersprite (`/Game/DataAssets/PrimaryDataAssets/Inventory/PDA_Base_InventoryItem.InventorySprite` _produceditem_itemdata))))))

(fn `UserConstructionScript`
  (`parent.UserConstructionScript`))

(fn `UseRecipe`
  (params (Inventory :type "/Game/Blueprints/Inventory/BP_Inventory Object Reference") (CheckingRecipe :type "/Game/DataAssets/PrimaryDataAssets/Crafting/PDA_CraftingRecipe Object Reference"))
  (locals (CurrentInvetory :type "/Game/Blueprints/Inventory/BP_Inventory Object Reference") (Recipe :type "/Game/DataAssets/PrimaryDataAssets/Crafting/PDA_CraftingRecipe Object Reference"))
  (bind _recipe (`local.Recipe`))
  (bind (_mainitem_itemdata _mainitem_itemamount) (break `/Game/DataAssets/PrimaryDataAssets/Inventory/SInventorySlot` (`/Game/DataAssets/PrimaryDataAssets/Crafting/PDA_CraftingRecipe.MainItem` _recipe)))
  (set `local.Recipe` CheckingRecipe)
  (bind _output_get (set `local.CurrentInvetory` Inventory))
  (`/Game/Blueprints/Inventory/BP_Inventory.RemoveItemByType` _output_get true _mainitem_itemdata _mainitem_itemamount)
  (for _array_element (`/Game/DataAssets/PrimaryDataAssets/Crafting/PDA_CraftingRecipe.SecondaryIngrediants` _recipe)
    (bind (_itemdata _itemamount) (break `/Game/DataAssets/PrimaryDataAssets/Inventory/SInventorySlot` _array_element))
    (`/Game/Blueprints/Inventory/BP_Inventory.RemoveItemByType` (`local.CurrentInvetory`) false _itemdata _itemamount)))