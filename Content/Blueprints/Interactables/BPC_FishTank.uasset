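; Interactable fish tank that simulates water chemistry for the fish and plants added to it.
; AddFish and AddPlant spawn actors at a downward-trace point and recompute oxygen and plant uptake rates.
; Tick derives live rates, chaining detritus and bacteria through the ammonia-nitrite-nitrate cycle, then integrates each stat over delta time.
; BeginPlay spawns randomly placed test fish into a boid manager; interaction shows the player's tank-stats UI.
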(event `self.ReceiveBeginPlay`
  (`parent.ReceiveBeginPlay`)
  (`/Engine/EditorBlueprintResources/StandardMacros.ForLoopConditional` 0 "NewEnumerator0" (`self.Test_FishToSpawn`)
    (:`LoopBody`
      (bind _returnvalue (`|SpawnActorFromClass` "/Game/Blueprints/Interactables/TankBlueprints/BP_Fish.BP_Fish_C" (`KismetMathLibrary.MakeTransform` (`KismetMathLibrary.MakeVector` (`KismetMathLibrary.RandomFloatInRange` -565.0 565.0) (`KismetMathLibrary.RandomFloatInRange` -535.0 535.0) (`KismetMathLibrary.RandomFloatInRange` -760.0 760.0))) "Undefined" "OverrideRootScale" null null))
      (`/Game/Blueprints/Interactables/TankBlueprints/BP_Fish.SetupFish` _returnvalue "/Game/DataAssets/Animals/AnimalDataAssets/DA_Entity_Fish_BoidTest_0.DA_Entity_Fish_BoidTest_0")
      (`/Game/Blueprints/Interactables/BaseBlueprints/BP_BoidManager.AddBoid` (`self.BP_BoidManager`) _returnvalue))))

(event `self.ReceiveTick`
  (params (DeltaSeconds :type "Float (single-precision)"))
  (`self.UpdateLiveRates`)
  (`self.CalculateAllStats` DeltaSeconds))

(event `self.PerformInteraction`
  (`parent.PerformInteraction`)
  (bind _asbp_player_char (cast `/Game/Character/BP_PlayerChar` (`GameplayStatics.GetPlayerCharacter` 0)))
  (bind _ui_tankstats (`/Game/Character/BP_PlayerChar.UI_TankStats` _asbp_player_char))
  (`UserWidget.AddToViewport` _ui_tankstats 0)
  (set `/Game/Blueprints/UI/UI_TankStats.CurrentTank` self _ui_tankstats))

(fn `Add Fish`
  (params (AnimalToAdd :type "/Game/DataAssets/PrimaryDataAssets/PDA_Animal Object Reference"))
  (returns (AnimalAdded :type Boolean))
  (bind (_returnvalue_location _returnvalue_rotation _returnvalue_scale) (`KismetMathLibrary.BreakTransform` (`self.GetTransform`)))
  (bind _returnvalue (`|SpawnActorFromClass` "/Game/Blueprints/Interactables/TankBlueprints/BP_Fish.BP_Fish_C" (`KismetMathLibrary.MakeTransform` (`self.GetTankViewLocation`) _returnvalue_rotation _returnvalue_scale) "AlwaysSpawn" "OverrideRootScale" null null))
  (bind _aspda_animal_fish (cast `/Game/DataAssets/PrimaryDataAssets/PDA_Animal_Fish` AnimalToAdd))
  (`/Game/Blueprints/Interactables/TankBlueprints/BP_Fish.SetupFish` _returnvalue _aspda_animal_fish)
  (`KismetArrayLibrary.Array_Add` (`self.AnimalsInTank`) _returnvalue)
  (`self.AdditionRates`)
  (return true))

(fn `AddDetritus`)

(fn `AdditionRates`
  (locals (TempCounter :type "Float (double-precision)") (TempCounter2 :type "Float (double-precision)") (TempCounter3 :type "Float (double-precision)"))
  (bind _lightlevel (`self.LightLevel`))
  (bind _tempcounter (`local.TempCounter`))
  (`|ExecutionSequence`
    (:`then_0`
      (for _array_element (`self.AnimalsInTank`)
        (set `local.TempCounter` (+ _tempcounter (`/Game/DataAssets/PrimaryDataAssets/PDA_Animal.OxygenUseRate` (`/Game/Blueprints/Interactables/TankBlueprints/BP_Fish.FishData` _array_element)))))
      (bind _output_get (set `self.OxygenRate(Out)` _tempcounter))
      (set `self.CO2Rate(In)` (* _output_get (`self.OxygenToCO2Rate`))))
    (:`then_1`
      (set `local.TempCounter` 0.0)
      (for _array_element_2 (`self.PlantsInTank`)
        (set `local.TempCounter` (+ (`local.TempCounter`) (`/Game/DataAssets/PrimaryDataAssets/PDA_Plant.GetNH3UseRate` _array_element_2 _lightlevel)))
        (set `local.TempCounter2` (+ (`local.TempCounter2`) (`/Game/DataAssets/PrimaryDataAssets/PDA_Plant.GetNitrateUseRate` _array_element_2 _lightlevel)))
        (set `local.TempCounter3` (+ (`local.TempCounter3`) (`/Game/DataAssets/PrimaryDataAssets/PDA_Plant.GetOxygenProductionRate` _array_element_2 _lightlevel))))
      (set `self.PlantAmmoniaRate` (`local.TempCounter`))
      (set `self.PlantNitrateRate` (`local.TempCounter2`))
      (set `self.PlantOxygenRate` (`local.TempCounter3`)))))

(fn `AddPlant`
  (params (PlantToAdd :type "/Game/DataAssets/PrimaryDataAssets/PDA_Plant Object Reference"))
  (returns (AnimalAdded :type Boolean))
  (bind (_returnvalue_location _returnvalue_rotation _returnvalue_scale) (`KismetMathLibrary.BreakTransform` (`self.GetTransform`)))
  (if (< (`KismetArrayLibrary.Array_Length` (`self.PlantActors`)) (`self.MaxPlantCount`))
    (bind _returnvalue (`|SpawnActorFromClass` "/Game/Blueprints/Interactables/TankBlueprints/BP_Plant.BP_Plant_C" (`KismetMathLibrary.MakeTransform` (`self.GetTankViewLocation`) _returnvalue_rotation _returnvalue_scale) "AlwaysSpawn" "OverrideRootScale" null null))
    (`KismetArrayLibrary.Array_Add` (`self.PlantActors`) _returnvalue)
    (`/Game/Blueprints/Interactables/TankBlueprints/BP_Plant.SetupPlant` _returnvalue PlantToAdd)
    (`self.K2_AttachToActor` _returnvalue self "None" "KeepWorld" "KeepWorld" "KeepWorld" true)
    (`KismetArrayLibrary.Array_Add` (`self.PlantsInTank`) PlantToAdd)
    (`self.AdditionRates`)
    (return true)
    (else
      (return false))))

(fn `CalculateAllStats`
  (params (Delta :type "Float (double-precision)"))
  (locals (DeltaTime :type "Float (double-precision)"))
  (set `local.DeltaTime` Delta)
  (bind _rescurrent (`self.CalculateStat` (`local.DeltaTime`) (`self.CurrentCO2`) (`self.CO2Rate(In)`) (`self.CO2Rate(Out)`)))
  (set `self.CurrentCO2` _rescurrent)
  (bind _rescurrent_2 (`self.CalculateStat` (`local.DeltaTime`) (`self.CurrentOxygen`) (`self.OxygenRate(In)`) (`self.OxygenRate(Out)`)))
  (set `self.CurrentOxygen` _rescurrent_2)
  (bind _rescurrent_3 (`self.CalculateStat` (`local.DeltaTime`) (`self.CurrentAmmonia`) (`self.AmmoniaRate(In)`) (`self.AmmoniaRate(Out)`)))
  (set `self.CurrentAmmonia` _rescurrent_3)
  (bind _rescurrent_4 (`self.CalculateStat` (`local.DeltaTime`) (`self.CurrentNitrites`) (`self.NitriteRate(In)`) (`self.NitriteRate(Out)`)))
  (set `self.CurrentNitrites` _rescurrent_4)
  (bind _rescurrent_5 (`self.CalculateStat` (`local.DeltaTime`) (`self.CurrentNitrates`) (`self.NitrateRate(In)`) (`self.NitrateRate(Out)`)))
  (set `self.CurrentNitrates` _rescurrent_5))

(fn `CalculateStat`
  (params (Time :type "Float (double-precision)") (Current :type "Float (double-precision)") (`In Rate` :type "Float (double-precision)") (`Out Rate` :type "Float (double-precision)"))
  (returns (ResCurrent :type "Float (double-precision)"))
  (return (- (+ (* Time `In Rate`) Current) (* `Out Rate` Time))))

(fn `GetTankStat`
  (params (StatType :type "/Game/DataAssets/Enums/Enum_TankStat Enum" :default "NewEnumerator0"))
  (returns (ReturnedStat :type "Float (double-precision)"))
  (switch `/Game/DataAssets/Enums/Enum_TankStat` StatType
    (:`NewEnumerator0`
      (return (`self.CurrentOxygen`)))
    (:`NewEnumerator1`
      (return (`self.CurrentCO2`)))
    (:`NewEnumerator2`
      (return (`self.CurrentAmmonia`)))
    (:`NewEnumerator3`
      (return (`self.MaxNitrites`)))
    (:`NewEnumerator4`
      (return (`self.CurrentNitrates`)))
    (:`NewEnumerator5`
      (return (`KismetMathLibrary.Conv_IntToDouble` (`self.CurrentDetritus`))))
    (:`NewEnumerator6`
      (return (`KismetMathLibrary.Conv_IntToDouble` (`self.LightLevel`))))))

(fn `GetTankViewLocation`
  (returns (Location :type "Vector Structure"))
  (bind (_returnvalue_x _returnvalue_y _returnvalue_z) (`KismetMathLibrary.BreakVector` (`SceneComponent.K2_GetComponentLocation` (`self.MovementPart`))))
  (bind (_outhit _returnvalue) (`KismetSystemLibrary.LineTraceSingle` :`Start` (`KismetMathLibrary.MakeVector` _returnvalue_x _returnvalue_y (+ _returnvalue_z 500.0)) :`End` (`KismetMathLibrary.MakeVector` _returnvalue_x _returnvalue_y (- _returnvalue_z 1000.0)) :`TraceChannel` "TraceTypeQuery4" :`bIgnoreSelf` false))
  (if _returnvalue
    (return (`.Location` (`GameplayStatics.BreakHitResult` _outhit)))
    (else
      (return (0.0 0.0 0.0)))))

(fn `StopInteraction`
  (bind _asbp_player_char (cast `/Game/Character/BP_PlayerChar` (`GameplayStatics.GetPlayerCharacter` 0)))
  (`Widget.RemoveFromParent` (`/Game/Character/BP_PlayerChar.UI_TankStats` _asbp_player_char)))

(fn `UpdateAmmoniaRate`
  (params (AmmoniaRate :type "Float (double-precision)"))
  (set `self.AmmoniaRate(In)` (+ AmmoniaRate (`self.AmmoniaRate(In)`))))

(fn `UpdateLiveRates`
  (`|ExecutionSequence`
    (:`then_0`
      (bind _output_get (set `self.OxygenRate(In)` (+ (`self.PlantOxygenRate`) (* (`self.OxygenRatePerDisturbance`) (`self.WaterDisturbance`)))))
      (set `self.CO2Rate(Out)` (* _output_get (`self.OxygenToCO2Rate`))))
    (:`then_1`
      (set `self.AmmoniaRate(In)` (* (`KismetMathLibrary.Conv_IntToDouble` (`self.CurrentDetritus`)) (`self.DetritusToAmmoniaRate`))))
    (:`then_2`
      (bind _output_get_2 (set `self.AmmoniaRate(Out)` (+ (`self.PlantAmmoniaRate`) (* (`KismetMathLibrary.Conv_IntToDouble` (`self.CurrentNitriteBacteria`)) (`self.AmmoniaToNitriteRate`)))))
      (set `self.NitriteRate(In)` (* _output_get_2 (`self.NitritePerAmmonia`))))
    (:`then_3`
      (bind _output_get_3 (set `self.NitriteRate(Out)` (* (`KismetMathLibrary.Conv_IntToDouble` (`self.CurrentNitrateBacteria`)) (`self.NitriteToNitrateRate`))))
      (set `self.NitrateRate(In)` (* _output_get_3 (`self.NitratePerNitrite`))))
    (:`then_4`
      (set `self.NitrateRate(Out)` (`self.PlantNitrateRate`)))))

(fn `UpdateOxygenRate`
  (params (OxygenRate :type "Float (double-precision)"))
  (set `self.OxygenRate(In)` (+ OxygenRate (`self.OxygenRate(In)`))))

(fn `UserConstructionScript`
  (`parent.UserConstructionScript`))