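; Interactable dispenser that gives a configured item to whoever interacts with it.
; The OnInteract event calls DispenseItem, which looks up a BP_Inventory component on the instigator and, if valid, adds ItemToAdd to it.
; Instigators without that component receive nothing, and the graph applies no stock limit or cooldown.
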(event `self.OnInteract`
  (params (Instigator :type "Actor Object Reference"))
  (`self.DispenseItem` Instigator))

(fn `DispenseItem`
  (params (Instigator :type "Actor Object Reference"))
  (bind _returnvalue (`self.GetComponentByClass` Instigator "/Game/Blueprints/Inventory/BP_Inventory.BP_Inventory_C"))
  (if (`KismetSystemLibrary.IsValid` _returnvalue)
    (`/Game/Blueprints/Inventory/BP_Inventory.AddItem` _returnvalue (`self.ItemToAdd`))))

(fn `UserConstructionScript`
  (`parent.UserConstructionScript`))