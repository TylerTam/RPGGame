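; Player character Blueprint that handles Enhanced Input movement, interaction and inventory, tracking facing for PaperZD.
; Interaction sphere-traces along the facing direction for BP_Interactable actors; cancelling stops the current one and blends the camera back.
; It creates runtime and full inventory widgets, relaying quick-select input and showing the selected item on HeldSprite.
; An enum-keyed map gates key actions, with bitmasks toggling input groups for menus and interactions.
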(event `self.ReceiveBeginPlay`
  (bind _asplayer_controller (cast `PlayerController` (`self.GetController`)))
  (`EnhancedInputSubsystemInterface.AddMappingContext` (pcsubsystem `EnhancedInputLocalPlayerSubsystem` _asplayer_controller) "/Game/Input/IMC_Player.IMC_Player" 0 (struct))
  (bind _returnvalue (`|CreateWidget` "/Game/Blueprints/UI/UI_TankStats.UI_TankStats_C"))
  (set `self.UI_TankStats` _returnvalue)
  (`self.SetupInventory`)
  (`self.SetupInputs`))

(event `self.ReceiveActorBeginOverlap`
  (params (OtherActor :type "Actor Object Reference")))

(event `EnhancedInput|/Game/Input/IA_Move`
  (params (ActionValue :type "Vector2D Structure") (ElapsedSeconds :type "Float (double-precision)") (TriggeredSeconds :type "Float (double-precision)") (InputAction :type "InputAction Object Reference" :default "/Game/Input/IA_Move.IA_Move"))
  (:`Triggered`
    (if (`self.IsInputEnabled` "NewEnumerator0") :!label _label
      (set `self.IsWalking` true)
      (`self.AddMovementInput` (1.0 0.0 0.0) ActionValue_X)
      (`self.AddMovementInput` (0.0 1.0 0.0) ActionValue_Y)
      (set `self.PaperZDDir` (`KismetMathLibrary.MakeVector2D` ActionValue_Y ActionValue_X))
      (set `self.FacingDr` (`KismetMathLibrary.MakeVector2D` ActionValue_X ActionValue_Y))
      (else
        (set `self.IsWalking` false :!label _label_2))))
  (:`Ongoing`
    (goto _label))
  (:`Completed`
    (goto _label_2)))

(event `EnhancedInput|/Game/Input/IA_Interact`
  (params (ActionValue :type Boolean) (ElapsedSeconds :type "Float (double-precision)") (TriggeredSeconds :type "Float (double-precision)") (InputAction :type "InputAction Object Reference" :default "/Game/Input/IA_Interact.IA_Interact"))
  (bind _returnvalue (`self.K2_GetActorLocation`))
  (bind _facingdr (`self.FacingDr`))
  (:`Started`
    (if (`self.IsInputEnabled` "NewEnumerator1")
      (bind (_outhit _returnvalue_2) (`KismetSystemLibrary.SphereTraceSingle` :`Start` (+ _returnvalue (* _facingdr (`self.InteractStartDis`))) :`End` (+ _returnvalue (* _facingdr (`self.InteractEndDis`))) :`Radius` 50.0 :`TraceChannel` "TraceTypeQuery3" :`DrawDebugType` "ForDuration" :`DrawTime` 0.1))
      (if _returnvalue_2
        (bind _asbp_interactable (cast `/Game/Blueprints/Interactables/BaseBlueprints/BP_Interactable` (`.HitActor` (`GameplayStatics.BreakHitResult` _outhit))))
        (if (`/Game/Blueprints/Interactables/BaseBlueprints/BP_Interactable.KeepInteractableRef` _asbp_interactable)
          (set `self.CurrentInteractable` _asbp_interactable))
        (`/Game/Blueprints/Interactables/BaseBlueprints/BP_Interactable.OnInteract` _asbp_interactable self)))))

(event `EnhancedInput|/Game/Input/IA_Cancel`
  (params (ActionValue :type Boolean) (ElapsedSeconds :type "Float (double-precision)") (TriggeredSeconds :type "Float (double-precision)") (InputAction :type "InputAction Object Reference" :default "/Game/Input/IA_Cancel.IA_Cancel"))
  (bind _currentinteractable (`self.CurrentInteractable`))
  (:`Started`
    (if (`KismetSystemLibrary.IsValid` _currentinteractable)
      (`/Game/Blueprints/Interactables/BaseBlueprints/BP_Interactable.StopInteraction` _currentinteractable)
      (`PlayerController.SetViewTargetWithBlend` (`GameplayStatics.GetPlayerController` 0) (`GameplayStatics.GetPlayerCharacter` 0) 1.0 "VTBlend_EaseInOut" 3.0 false)
      (set `self.CurrentInteractable` null)
      (`KismetSystemLibrary.Delay` 1.0)
      (`self.Toggle Inputs` true (`self.DisableOnInteract`)))))

(event `SelectedInventoryItemChanged`
  (params (NewItem :type "/Game/DataAssets/PrimaryDataAssets/Inventory/PDA_Base_InventoryItem Object Reference"))
  (bind _heldsprite (`self.HeldSprite`))
  (if (`KismetSystemLibrary.IsValid` NewItem)
    (`SceneComponent.SetVisibility` _heldsprite true false)
    (`PaperSpriteComponent.SetSprite` _heldsprite (`/Game/DataAssets/PrimaryDataAssets/Inventory/PDA_Base_InventoryItem.InventorySprite` NewItem))
    (else
      (`SceneComponent.SetVisibility` _heldsprite false false))))

(event `EnhancedInput|/Game/Input/IA_QuickSelectDir`
  (params (ActionValue :type "Float (double-precision)") (ElapsedSeconds :type "Float (double-precision)") (TriggeredSeconds :type "Float (double-precision)") (InputAction :type "InputAction Object Reference" :default "/Game/Input/IA_QuickSelectDir.IA_QuickSelectDir"))
  (:`Triggered`
    (`self.ItemDirChange` (`KismetMathLibrary.FTrunc` (`KismetMathLibrary.SignOfFloat` ActionValue)))))

(event `EnhancedInput|/Game/Input/IA_QuickSelectRow`
  (params (ActionValue :type "Float (double-precision)") (ElapsedSeconds :type "Float (double-precision)") (TriggeredSeconds :type "Float (double-precision)") (InputAction :type "InputAction Object Reference" :default "/Game/Input/IA_QuickSelectRow.IA_QuickSelectRow"))
  (:`Triggered`
    (`self.ItemRowChange` (`KismetMathLibrary.FTrunc` (`KismetMathLibrary.SignOfFloat` ActionValue)))))

(event `EnhancedInput|/Game/Input/IA_UseSelected`
  (params (ActionValue :type Boolean) (ElapsedSeconds :type "Float (double-precision)") (TriggeredSeconds :type "Float (double-precision)") (InputAction :type "InputAction Object Reference" :default "/Game/Input/IA_UseSelected.IA_UseSelected"))
  (:`Triggered`
    (if (`self.IsInputEnabled` "NewEnumerator4")
      (`/Game/Blueprints/UI/UI_InventoryRuntime.UseSelectedItem` (`self.InventoryRuntime`) (`self.CurrentInteractable`)))))

(event `EnhancedInput|/Game/Input/IA_OpenInventory`
  (params (ActionValue :type Boolean) (ElapsedSeconds :type "Float (double-precision)") (TriggeredSeconds :type "Float (double-precision)") (InputAction :type "InputAction Object Reference" :default "/Game/Input/IA_OpenInventory.IA_OpenInventory"))
  (:`Triggered`
    (bind _isopen (`/Game/Blueprints/UI/UI_Inventory.ToggleUI` (`self.InventoryUI`)))
    (`self.Toggle Inputs` (not _isopen) (`self.DisableOnMenu`))))

(fn `GetSelectedItem`
  (returns (Item :type "/Game/DataAssets/PrimaryDataAssets/Inventory/PDA_Base_InventoryItem Object Reference"))
  (bind _item (`/Game/Blueprints/UI/UI_InventoryRuntime.GetSelectedItem` (`self.InventoryRuntime`)))
  (return _item))

(fn `IsInputEnabled`
  (params (InputType :type "/Game/DataAssets/Enums/Enum_Input Enum" :default "NewEnumerator0"))
  (returns (Enabled :type Boolean))
  (return (`BlueprintMapLibrary.Map_Find` (`self.Inputs`) InputType)))

(fn `SetupInputs`
  (bind _enumvalue (foreach `/Game/DataAssets/Enums/Enum_Input` true)
    (:`LoopBody`
      (`BlueprintMapLibrary.Map_Add` (`self.Inputs`) _enumvalue))
    (:`then`
      (`self.Toggle Inputs` true (`self.InitialEnabledInputs`)))))

(fn `SetupInventory`
  (bind _returnvalue (`|CreateWidget` "/Game/Blueprints/UI/UI_InventoryRuntime.UI_InventoryRuntime_C"))
  (bind _output_get (set `self.InventoryRuntime` _returnvalue))
  (`/Game/Blueprints/UI/UI_InventoryRuntime.SetupUI` _output_get (`self.BP_Inventory`))
  (`UserWidget.AddToViewport` _output_get 0)
  (add `/Game/Blueprints/UI/UI_InventoryRuntime.SelectedChanged` _output_get (`|CreateDelegate` :!event `SelectedInventoryItemChanged`))
  (add `self.ItemDirChange` (`|CreateDelegate` _output_get :!event `ChangeIndex`))
  (add `self.ItemRowChange` (`|CreateDelegate` _output_get :!event `ChangeRow`))
  (bind _returnvalue_2 (`|CreateWidget` "/Game/Blueprints/UI/UI_Inventory.UI_Inventory_C"))
  (bind _output_get_2 (set `self.InventoryUI` _returnvalue_2))
  (`/Game/Blueprints/UI/UI_Inventory.SetupUI` _output_get_2 (`self.BP_Inventory`))
  (`UserWidget.AddToViewport` _output_get_2 0)
  (`Widget.SetVisibility` _output_get_2 "Collapsed"))

(fn `Toggle Inputs`
  (params (Enable :type Boolean) (BitmaskInputs :type Integer))
  (bind _enumvalue (foreach `/Game/DataAssets/Enums/Enum_Input` false)
    (:`LoopBody`
      (if (`KismetMathLibrary.Conv_IntToBool` (`KismetMathLibrary.And_IntInt` BitmaskInputs (`KismetMathLibrary.FFloor` (`KismetMathLibrary.MultiplyMultiply_FloatFloat` 2.0 (`KismetMathLibrary.Conv_ByteToDouble` _enumvalue)))))
        (`BlueprintMapLibrary.Map_Add` (`self.Inputs`) _enumvalue Enable)))))

(fn `ToggleInput`
  (params (InputType :type "/Game/DataAssets/Enums/Enum_Input Enum" :default "NewEnumerator0") (Enable :type Boolean))
  (`BlueprintMapLibrary.Map_Add` (`self.Inputs`) InputType Enable))

(fn `UserConstructionScript`)